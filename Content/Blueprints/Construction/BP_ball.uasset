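; BP_ball is a ball actor that travels in a straight line and bounces off whatever blocks it, slowing with each bounce.
; Each Tick sweeps it along Direction at Speed, and a blocking hit reflects Direction about the hit normal.
; Each bounce also subtracts a tenth of the speed saved at BeginPlay, skipping the reduction if it would fall below MinimalSpeed.
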(event `self.ReceiveBeginPlay`
  (set `self.initial_speed` (`self.speed`)))

(event `self.ReceiveTick`
  (params (DeltaSeconds :type "Float (single-precision)"))
  (bind _returnvalue (- (`self.speed`) (`KismetMathLibrary.SafeDivide` (`self.initial_speed`) 10.0)))
  (bind _sweephitresult (`self.K2_AddActorWorldOffset` (* (* (`self.Direction`) (`self.speed`)) DeltaSeconds) true))
  (bind (_bblockinghit _binitialoverlap _time _distance _location _impactpoint _normal) (`GameplayStatics.BreakHitResult` _sweephitresult))
  (if _bblockinghit
    (set `self.Direction` (`KismetMathLibrary.GetReflectionVector` (`self.Direction`) _normal))
    (`/Engine/EditorBlueprintResources/StandardMacros.CompareFloat` _returnvalue (`self.minimal_speed`)
      (:`>`
        _)
      (:`==`
        _))
    (set `self.speed` _returnvalue)))

(fn `UserConstructionScript`)